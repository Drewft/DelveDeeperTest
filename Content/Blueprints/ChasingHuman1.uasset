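; ChasingHuman1 is an enemy pawn that chases the player and ends the game in a loss on contact.
; On BeginPlay, a custom CHASING event issues a single AI MoveTo on itself, targeting the player controller rather than the player pawn.
; When an actor tagged Player overlaps its Cylinder component, it prints a death message and calls Lose on BP_FirstPersonGameMode.
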(event `self.ReceiveBeginPlay`
  (`self.CHASING`))

(event `CHASING`
  (`|ExecutionSequence`
    (:`then_0`
      (`|AIMoveTo` self (0.0 0.0 0.0) (`GameplayStatics.GetPlayerController` 0)))))

(event `self.ReceiveTick`
  (params (DeltaSeconds :type "Float (single-precision)")))

(event `self.Cylinder.OnComponentBeginOverlap`
  (params (OverlappedComponent :type "PrimitiveComponent Object Reference") (OtherActor :type "Actor Object Reference") (OtherComp :type "PrimitiveComponent Object Reference") (OtherBodyIndex :type Integer) (bFromSweep :type Boolean) (SweepResult :type "HitResult Structure (by ref)"))
  (if (`self.ActorHasTag` OtherActor "Player")
    (bind _asbp_first_person_game_mode (cast `/Game/FirstPerson/Blueprints/BP_FirstPersonGameMode` (`GameplayStatics.GetGameMode`)))
    (`KismetSystemLibrary.PrintString` "YUou're dead!")
    (`/Game/FirstPerson/Blueprints/BP_FirstPersonGameMode.Lose` _asbp_first_person_game_mode)))

(fn `UserConstructionScript`)