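; Patrolling human enemy that walks a looping route through four points and ends the game if it catches the player after spotting them.
; Chained AI MoveTo calls drive the patrol, restarting only when every leg succeeds.
; PawnSensing permanently sets Seen and issues a move toward the player controller, rather than its pawn.
; Cylinder overlaps by any actor while Seen call the game mode's Lose, while clicking the Cube destroys the human.
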(event `self.ReceiveBeginPlay`
  (`self.Movearound`))

(event `Die`
  (`self.K2_DestroyActor`))

(event `Movearound`
  (`|AIMoveTo` self (`self.Point1`) null
    (:`OnSuccess`
      (`|AIMoveTo` self (`self.Point2`) null
        (:`OnSuccess`
          (`|AIMoveTo` self (`self.Point3`) null
            (:`OnSuccess`
              (`|AIMoveTo` self (`self.Point4`) null
                (:`OnSuccess`
                  (`self.Movearound`))))))))))

(event `self.PawnSensing.OnSeePawn`
  (params (Pawn :type "Pawn Object Reference"))
  (if true
    (set `self.Seen` true)
    (`self.FollowPlayer`)))

(event `FollowPlayer`
  (if (`self.Seen`)
    (`KismetSystemLibrary.PrintString` "I SEE YOU")
    (`|AIMoveTo` self (0.0 0.0 0.0) (`GameplayStatics.GetPlayerController` 0))))

(event `self.Cube.OnClicked`
  (params (TouchedComponent :type "PrimitiveComponent Object Reference") (ButtonPressed :type "Key Structure"))
  (`KismetSystemLibrary.PrintString` "Dead  ")
  (`self.K2_DestroyActor`))

(event `self.Cylinder.OnComponentBeginOverlap`
  (params (OverlappedComponent :type "PrimitiveComponent Object Reference") (OtherActor :type "Actor Object Reference") (OtherComp :type "PrimitiveComponent Object Reference") (OtherBodyIndex :type Integer) (bFromSweep :type Boolean) (SweepResult :type "HitResult Structure (by ref)"))
  (if (`self.Seen`)
    (`KismetSystemLibrary.PrintString` "Hello")
    (bind _asbp_first_person_game_mode (cast `/Game/FirstPerson/Blueprints/BP_FirstPersonGameMode` (`GameplayStatics.GetGameMode`)))
    (`KismetSystemLibrary.PrintString` "YUou're dead!")
    (`/Game/FirstPerson/Blueprints/BP_FirstPersonGameMode.Lose` _asbp_first_person_game_mode)))

(fn `UserConstructionScript`)