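; A security camera that sweeps its view and raises an alarm when the player enters its detection cone.
; A timeline started on BeginPlay drives the yaw of CameraCube at a fixed downward pitch.
; Cone overlap by a Player-tagged actor flashes the spot and point lights red, then calls KameraFollow on PatrollingHuman4 actors found by class.
; After a delay, the lights turn orange; debug prints report success or failure.
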(event `self.ReceiveBeginPlay`
  (`self.CameraRotate`))

(event `CameraRotate`
  (bind (_direction _camerarotation) (`Timeline|Timeline`)
    (:`Update`
      (`SceneComponent.K2_SetRelativeRotation` (`self.Camera_Cube`) (`KismetMathLibrary.MakeRotator` 0.0 -20.0 _camerarotation) false false))))

(event `self.Cone.OnComponentBeginOverlap`
  (params (OverlappedComponent :type "PrimitiveComponent Object Reference") (OtherActor :type "Actor Object Reference") (OtherComp :type "PrimitiveComponent Object Reference") (OtherBodyIndex :type Integer) (bFromSweep :type Boolean) (SweepResult :type "HitResult Structure (by ref)"))
  (if (`self.ActorHasTag` OtherActor "Player")
    (`KismetSystemLibrary.PrintString` "Success!")
    (`LightComponent.SetLightColor` (`self.SpotLight`) (struct :`R` 1.0 :`A` 1.0) true)
    (`LightComponent.SetLightColor` (`self.PointLight`) (struct :`R` 1.0 :`A` 1.0) true)
    (`KismetSystemLibrary.Delay` 0.4)
    (`LightComponent.SetLightColor` (`self.SpotLight`) (struct :`A` 1.0) true)
    (`LightComponent.SetLightColor` (`self.PointLight`) (struct :`A` 1.0) true)
    (`KismetSystemLibrary.Delay` 0.4)
    (`LightComponent.SetLightColor` (`self.SpotLight`) (struct :`R` 1.0 :`A` 1.0) true)
    (`LightComponent.SetLightColor` (`self.PointLight`) (struct :`R` 1.0 :`A` 1.0) true)
    (`KismetSystemLibrary.Delay` 0.4)
    (bind _aspatrolling_human_4 (castclass `/Game/Blueprints/PatrollingHuman4` "/Game/Blueprints/PatrollingHuman4.PatrollingHuman4_C"))
    (bind _outactors (`GameplayStatics.GetAllActorsOfClass` _aspatrolling_human_4))
    (`/Game/Blueprints/PatrollingHuman4.KameraFollow` _outactors)
    (`KismetSystemLibrary.Delay` 5.0)
    (`LightComponent.SetLightColor` (`self.SpotLight`) (struct :`R` 1.0 :`G` 0.5 :`A` 1.0) true)
    (`LightComponent.SetLightColor` (`self.PointLight`) (struct :`R` 1.0 :`G` 0.5 :`A` 1.0) true)
    (else
      (`KismetSystemLibrary.PrintString` "Fail!"))))

(fn `UserConstructionScript`)